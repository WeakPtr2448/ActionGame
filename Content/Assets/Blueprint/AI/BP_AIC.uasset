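; Enemy AI controller that runs the BT_Enemy behavior tree and targets player-controlled pawns it senses.
; On begin play it starts the tree, then perception updates drive the Blackboard Target, controller focus and a SetLockTarget message to the controlled pawn.
; Any failed-sense update clears all three, whichever actor was lost.
; A disconnected AIMoveTo test toward the player never runs.
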(event OnTargetPerceptionUpdated(AIPerception)
  (params (Actor :type Actor%20Object%20Reference) (Stimulus :type AI%20Stimulus%20Structure))
  (if (Utilities|Struct|BreakAIStimulus Stimulus)
    (bind _aspawn (Utilities|Casting|CastToPawn Actor))
    (if (Pawn|IsPlayerControlled _aspawn)
      (AI|Components|Blackboard|SetValueasObject (Variables|Default|GetBlackboard) (Utilities|Name|MakeLiteralName "Target") Actor)
      (AI|SetFocus Actor)
      (Class|ICharacterAttrs|SetLockTarget(Message) (Pawn|GetControlledPawn) _aspawn))
    (else
      (AI|Components|Blackboard|SetValueasObject (Variables|Default|GetBlackboard) (Utilities|Name|MakeLiteralName "Target") 0)
      (AI|SetFocus)
      (Class|ICharacterAttrs|SetLockTarget(Message) (Pawn|GetControlledPawn)))))

(event EventBeginPlay
  (AI|RunBehaviorTree "/Game/Assets/Blueprint/AI/BT_Enemy.BT_Enemy"))

(event EventTick
  (params (DeltaSeconds :type Float%20%28single-precision%29)))

(fn ConstructionScript)