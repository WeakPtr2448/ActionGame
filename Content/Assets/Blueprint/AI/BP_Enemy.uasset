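; BP_Enemy is an enemy Blueprint with hooks for lock-on display and targeting.
; SetLockUIVisibility shows or hides the LockWidgetComp widget.
; SetLockTarget clears LockTargetActors and writes in the given pawn, so the array holds only that one target.
; The graphs contain no other active logic, as BeginPlay, overlap and Tick are disabled stubs.
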(event EventBeginPlay
  (|CallParentFunction) ; This node is disabled and will not be called.\nDrag off pins to build functionality.
)

(event Collision|EventActorBeginOverlap
  (params (OtherActor :type Actor%20Object%20Reference))
  (|CallParentFunction OtherActor) ; This node is disabled and will not be called.\nDrag off pins to build functionality.
)

(event EventTick
  (params (DeltaSeconds :type Float%20%28single-precision%29))
  (|CallParentFunction DeltaSeconds) ; This node is disabled and will not be called.\nDrag off pins to build functionality.
)

(event EventSetLockUIVisibility
  (params (InVisibility :type Boolean))
  (Rendering|SetVisibility (Variables|Default|GetLockWidgetComp) InVisibility false))

(event EventSetLockTarget
  (params (TargetPawn :type Actor%20Object%20Reference))
  (bind _locktargetactors (Variables|Default|GetLockTargetActors))
  (Utilities|Array|Clear _locktargetactors)
  (Utilities|Array|SetArrayElem _locktargetactors 0 TargetPawn true))

(fn ConstructionScript
  (|CallParentFunction))