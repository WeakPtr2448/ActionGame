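; Base action-combat character with walk/run, directional rolls, weapon toggling through montages and material fades, and saber combos.
; Attacks run looping timer box traces between saber sockets, triggering thunder VFX, directional hit reactions and, for players, hit-stop and camera shake.
; An overlap volume gathers lock-on targets, which can be cycled; Tick turns character and controller toward the selected one and eases spring-arm length.
; Input-buffer command matching is unfinished and disconnected.
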(event OnComponentBeginOverlap(LockTargetCollision)
  (params (OverlappedComponent :type Primitive%20Component%20Object%20Reference) (OtherActor :type Actor%20Object%20Reference) (OtherComp :type Primitive%20Component%20Object%20Reference) (OtherBodyIndex :type Integer) (bFromSweep :type Boolean) (SweepResult :type Hit%20Result%20Structure%20%28by%20ref%29))
  ;[1 1 1] UpdateLockTargets
  (bind _aspawn (Utilities|Casting|CastToPawn OtherActor))
  (Utilities|Array|Add (Variables|Default|GetLockTargetActors) _aspawn)
  (UI|SwitchLockTargetUI))

(event OnComponentEndOverlap(LockTargetCollision)
  (params (OverlappedComponent :type Primitive%20Component%20Object%20Reference) (OtherActor :type Actor%20Object%20Reference) (OtherComp :type Primitive%20Component%20Object%20Reference) (OtherBodyIndex :type Integer))
  ;[1 1 1] UpdateLockTargets
  (if (Utilities|IsValidLockTargetArray)
    (if (Utilities|Array|ContainsItem (Variables|Default|GetLockTargetActors) OtherActor)
      (Class|ICharacterAttrs|SetLockUIVisibility(Message) OtherActor false)
      (Utilities|Array|RemoveItem (Variables|Default|GetLockTargetActors) OtherActor)
      (UI|SwitchLockTargetUI))))

(event Custom|SpawnEffect
  ;[1 0 0.8168] 花里胡哨的特效
  (bind _appearance (Timeline|EffectTimeline Play)
    (:Update
      (Rendering|Material|SetScalarParameterValue (Variables|Material|GetSkinMatDynamic) "Appearance" _appearance :!class /Script/Engine.MaterialInstanceDynamic))
    (:Finished
      (Components|Activation|SetActive (Variables|Default|GetNS_ky_aura_ice) false false))))

(event EventBeginPlay
  ;[0.2602 1 0.8801] Beginplay
  (Utilities|FlowControl|Sequence
    (:then_0
      (Utilities|Array|Clear (Variables|Default|GetHitActors))
      (Variables|Action|SetCurrentRotation (Transformation|GetActorRotation))
      (Rendering|Material|SetScalarParameterValue (Variables|Material|GetWeaponSkinMatDynamic) "Appearance" 1.0 :!class /Script/Engine.MaterialInstanceDynamic)
      (Variables|Default|SetCurrentArmLength (Variables|/Script/Engine.SpringArmComponent|GetTargetArmLength (Variables|Default|GetSpringArm))))
    (:then_1
      (CallFunction|SpawnEffect))
    (:then_2
      (Utilities|Array|Clear (Variables|Default|GetLockTargetActors)))
    (:then_3
      (CameraFades|StartCameraFade (Game|GetPlayerCameraManager 0) 1.0 0.0 5.0 "(R=0.000000,G=0.000000,B=0.000000,A=1.000000)" false false))))

(event Collision|EventActorBeginOverlap
  (params (OtherActor :type Actor%20Object%20Reference)))

(event EventTick
  (params (DeltaSeconds :type Float%20%28single-precision%29))
  (bind _charactermovement (Variables|Character|GetCharacterMovement))
  ;[1 1 1] Tick
  (Utilities|FlowControl|Sequence
    (:then_0
      (if (or (!= (Input|AxisValues|GetMoveForward) 0.0) (!= (Input|AxisValues|GetMoveRight) 0.0))
        (Variables|/Script/Engine.CharacterMovementComponent|SetbUseControllerDesiredRotation _charactermovement true)
        (else
          (Variables|/Script/Engine.CharacterMovementComponent|SetbUseControllerDesiredRotation _charactermovement false))))
    (:then_1
      (CallFunction|MakeCharacterOrienttoHitActor :!pinned true) ; 让角色始终朝向锁定的目标
    )
    (:then_2
      (if (Pawn|IsPlayerControlled)
        (CallFunction|UpdateSpringArmLength (select (Utilities|IsValidLockTargetArray) 7e+02 3.5e+02) 1.0 :!pinned true) ; 更新弹簧臂长度
      ))))

(event Input|KeyboardEvents|1
  (params (Key :type Key%20Structure :default "None"))
  (bind _effecttimeline (Variables|Default|GetEffectTimeline))
  ;[1 1 1] Test
  (:Pressed
    (Utilities|FlowControl|FlipFlop
      (:A
        (Utilities|String|Reverse _effecttimeline))
      (:B
        (Audio|Components|Audio|Play _effecttimeline)))))

(fn ConstructionScript
  (Utilities|FlowControl|Sequence
    (:then_0
      (bind _returnvalue (Rendering|Material|CreateDynamicMaterialInstance (Variables|Character|GetMesh) 0 (Variables|Material|GetSource%20Material) "None" :!class /Script/Engine.PrimitiveComponent))
      (Variables|Material|SetSkinMatDynamic _returnvalue))
    (:then_1
      (bind _returnvalue_2 (Rendering|Material|CreateDynamicMaterialInstance (Variables|Default|GetSaber) 0 "/Game/Assets/Material/MI_Sword.MI_Sword" "None" :!class /Script/Engine.PrimitiveComponent))
      (Variables|Material|SetWeaponSkinMatDynamic _returnvalue_2))))

(fn CalculateDir
  (params (InVector :type Vector))
  (LocalVariables|SetDegree (Class|KismetMathLibrary|DegAcos (Math|Vector|DotProduct (Math|Vector|Normalize InVector) (Transformation|GetActorForwardVector))))
  (if (< (Math|Float|Sign(Float) (.Z (Math|Vector|BreakVector (Math|Vector|CrossProduct (Transformation|GetActorForwardVector) (Math|Vector|Normalize InVector))))) 0.0)
    (LocalVariables|SetDegree (* (LocalVariables|GetDegree) -1.0)))
  (return (LocalVariables|GetDegree)))

(fn CalculateDirection
  (params (InVector :type Vector) (BaseRotation :type Rotator))
  (LocalVariables|SetAngle%28Local%29 (Class|KismetMathLibrary|DegAcos (Math|Vector|DotProduct (Math|Vector|Normalize InVector) (Math|Vector|GetForwardVector BaseRotation))))
  (if (< (Math|Float|Sign(Float) (.Z (Math|Vector|BreakVector (Math|Vector|CrossProduct (Math|Vector|GetForwardVector BaseRotation) (Math|Vector|Normalize InVector))))) 0.0)
    (LocalVariables|SetAngle%28Local%29 (* (LocalVariables|GetAngle%28Local%29) -1.0))
    (elif (== (Math|Vector|VectorLength InVector) 0.0)
      (LocalVariables|SetAngle%28Local%29 0.0)))
  (return (LocalVariables|GetAngle%28Local%29)))

(fn PlayHitAnimation
  (params (InCharacter :type Character%20Object%20Reference) (HitNormal :type Vector))
  (bind _outdegree (CallFunction|CalculateDir HitNormal))
  (if (Math|Float|InRange(Float) _outdegree -45.0 45.0 false false)
    (Variables|Action|State|SetHitDirection "NewEnumerator0")
    (elif (Math|Float|InRange(Float) _outdegree -135.0 -45.0 false)
      (Variables|Action|State|SetHitDirection "NewEnumerator2")
      (elif (Math|Float|InRange(Float) _outdegree 45.0 135.0 true false)
        (Variables|Action|State|SetHitDirection "NewEnumerator3")
        (else
          (Variables|Action|State|SetHitDirection "NewEnumerator1")))))
  (bind _incharacter (LocalVariables|GetInCharacter)
    (:then
      (Animation|Montage|MontagePlay (Components|SkeletalMesh|GetAnimInstance (Variables|/Script/Engine.Character|GetMesh _incharacter)) (Utilities|Select :Index (Variables|Action|State|GetHitDirection) :NewEnumerator0 "/Game/Assets/Sword_Animations/Animations/Sequence/08_Hit/05_Hit_Large/AM_Hit_Large_F_Seq.AM_Hit_Large_F_Seq" :NewEnumerator1 "/Game/Assets/Sword_Animations/Animations/Sequence/08_Hit/05_Hit_Large/AM_Hit_Large_B_Seq.AM_Hit_Large_B_Seq" :NewEnumerator2 "/Game/Assets/Sword_Animations/Animations/Sequence/08_Hit/05_Hit_Large/AM_Hit_Large_L_Seq.AM_Hit_Large_L_Seq" :NewEnumerator3 "/Game/Assets/Sword_Animations/Animations/Sequence/08_Hit/05_Hit_Large/AM_Hit_Large_R_Seq.AM_Hit_Large_R_Seq") 1.0 "MontageLength" 0.0 true))
    (:else)))

(fn MakeCharacterOrienttoHitActor
  (if (> (Utilities|Array|Length (Variables|Default|GetLockTargetActors)) 0)
    (Utilities|IsValid (Utilities|Array|Get(acopy) (Variables|Default|GetLockTargetActors) (Variables|Default|GetLockTargetIndex))
      (:Is%20Valid
        (bind _output_get (Variables|Action|SetCurrentRotation (Math|Interpolation|RInterpTo (Variables|Action|GetCurrentRotation) (Math|Rotator|FindLookatRotation (Transformation|GetActorLocation) (Transformation|GetActorLocation (Utilities|Array|Get(acopy) (Variables|Default|GetLockTargetActors) (Variables|Default|GetLockTargetIndex)))) (Utilities|Time|GetWorldDeltaSeconds) 6.0)))
        (Transformation|SetActorRotation (Math|Rotator|MakeRotator (.Roll (Math|Rotator|BreakRotator _output_get)) 0.0 (.Yaw (Math|Rotator|BreakRotator _output_get))))
        (Pawn|SetControlRotation (Pawn|GetController) (Math|Rotator|MakeRotator (.Roll (Math|Rotator|BreakRotator _output_get)) (.pitch (Pawn|GetControlRotation :!class /Script/Engine.Pawn)) (.Yaw (Math|Rotator|BreakRotator _output_get))))))))

(fn UpdateSpringArmLength
  (params (Target :type Float%20%28single-precision%29) (InterpSpeed :type Float%20%28single-precision%29))
  (bind _output_get (Variables|Default|SetCurrentArmLength (Math|Interpolation|FInterpTo (Variables|Default|GetCurrentArmLength) Target (Utilities|Time|GetWorldDeltaSeconds) InterpSpeed)))
  (Variables|/Script/Engine.SpringArmComponent|SetTargetArmLength (Variables|Default|GetSpringArm) _output_get))

(fn SwitchLockTargetUI
  (bind _locktargetactors (Variables|Default|GetLockTargetActors))
  (if (Pawn|IsPlayerControlled)
    (if (Utilities|IsValidLockTargetArray)
      (for _array_element _locktargetactors
        (Class|ICharacterAttrs|SetLockUIVisibility(Message) _array_element (== _array_element (Utilities|Array|Get(acopy) _locktargetactors (Variables|Default|GetLockTargetIndex))))))))

(fn CalculateRollDirection
  (return (.Yaw (Math|Rotator|BreakRotator (Math|Rotator|Delta(Rotator) (Math|Conversions|RotationFromXVector (+ (* (Transformation|GetActorForwardVector) (select (or (!= (Input|AxisValues|GetMoveForward) 0.0) (!= (Input|AxisValues|GetMoveRight) 0.0)) (Input|AxisValues|GetMoveForward) -1.0)) (* (Transformation|GetActorRightVector) (select (or (!= (Input|AxisValues|GetMoveRight) 0.0) (!= (Input|AxisValues|GetMoveForward) 0.0)) (Input|AxisValues|GetMoveRight) 0.0)))) (Transformation|GetActorRotation))))))

(fn CheckInputCommand
  (params (CommandInput :type S%20Input%20Buffer%20Structure))
  (bind _inputbuffers (Variables|Command|GetInputBuffers))
  (Utilities|Array|Add (Variables|Command|GetInputBuffers) CommandInput)
  (for (_array_element _array_index) (.InputKeys (Utilities|Struct|BreakS_Command (Utilities|Array|Get(acopy) (Variables|Command|GetCommands))))
    (for (_ _array_index_2) _inputbuffers
      (Development|PrintString (.InputKeyName (Utilities|Struct|BreakS_InputBuffer (Utilities|Array|Get(acopy) _inputbuffers (+ _array_index_2 (Variables|Default|GetCount))))))
      (if (Utilities|Enum|Equal(Enum) (Utilities|String|ToString(Text) (Class|KismetInputLibrary|KeyGetDisplayName _array_element)) (.InputKeyName (Utilities|Struct|BreakS_InputBuffer (Utilities|Array|Get(acopy) _inputbuffers (+ _array_index_2 (Variables|Default|GetCount))))))
        (Math|Integer|IncrementInt (Variables|Default|GetCount)
          (:%20%20
            (Development|PrintString (Utilities|String|ToString(Integer) (Variables|Default|GetCount)) true false "(R=1.000000,G=0.118055,B=0.000000,A=1.000000)" 5.0)))
        (else
          (Variables|Default|SetCount 0)
          (return))))))

(fn GetAttackKeyDown
  (return (Variables|Action|GetbAttackKeyDown)))

(fn GetCurrentState
  (return (Variables|Action|State|GetCurrentState)))

(fn GetIsRunning
  (return (Variables|Action|GetbIsRunning)))

(fn GetMoveValue
  (return (Math|Vector2D|MakeVector2D (Input|AxisValues|GetMoveForward) (Input|AxisValues|GetMoveRight))))

(event Input|AxisEvents|InputAxisMoveForward
  (params (AxisValue :type Float%20%28single-precision%29))
  (Pawn|Input|AddMovementInput (Math|Vector|GetForwardVector (Math|Rotator|MakeRotator 0.0 0.0 (.Yaw (Math|Rotator|BreakRotator (Pawn|GetControlRotation :!class /Script/Engine.Pawn))))) AxisValue false))

(event Input|AxisEvents|InputAxisMoveRight
  (params (AxisValue :type Float%20%28single-precision%29))
  (Pawn|Input|AddMovementInput (Math|Vector|GetRightVector (Math|Rotator|MakeRotator 0.0 0.0 (.Yaw (Math|Rotator|BreakRotator (Pawn|GetControlRotation :!class /Script/Engine.Pawn))))) AxisValue false))

(event Input|AxisEvents|InputAxisTurn
  (params (AxisValue :type Float%20%28single-precision%29))
  (Pawn|Input|AddControllerYawInput AxisValue))

(event Input|AxisEvents|InputAxisLookUp
  (params (AxisValue :type Float%20%28single-precision%29))
  (Pawn|Input|AddControllerPitchInput AxisValue))

(event EventSetCurrentState
  (params (NewState :type E_CharacterState%20Enum :default "NewEnumerator0"))
  (Variables|Action|State|SetCurrentState NewState))

(event EventSwitchWeapon
  (switch Utilities|FlowControl|Switch|SwitchonE_CharacterState (Variables|Action|State|GetCurrentState)
    (:NewEnumerator0
      (Animation|Montage|MontagePlay (Components|SkeletalMesh|GetAnimInstance (Variables|Character|GetMesh)) "/Game/Assets/Sword_Animations/Animations/Sequence/01_Idle/AM_Idle_To_Idle_Combat_Seq.AM_Idle_To_Idle_Combat_Seq" 1.0 "MontageLength" 0.0 true)
      (bind _visible (Timeline|WeaponVisibleTimeline Play)
        (:Update
          (Rendering|Material|SetScalarParameterValue (Variables|Material|GetWeaponSkinMatDynamic) "Appearance" _visible :!class /Script/Engine.MaterialInstanceDynamic))))
    (:NewEnumerator1
      (Animation|Montage|MontagePlay (Components|SkeletalMesh|GetAnimInstance (Variables|Character|GetMesh)) "/Game/Assets/Sword_Animations/Animations/Sequence/01_Idle/AM_Idle_Combat_To_Idle_Seq.AM_Idle_Combat_To_Idle_Seq" 1.0 "MontageLength" 0.0 true)
      (Timeline|WeaponVisibleTimeline Reverse))))

(event Input|ActionEvents|InputActionToggleWeapon
  (params (Key :type Key%20Structure :default "None"))
  (:Pressed
    (switch Utilities|FlowControl|Switch|SwitchonE_CharacterState (Variables|Action|State|GetCurrentState)
      (:NewEnumerator0
        (Animation|Montage|MontagePlay (Components|SkeletalMesh|GetAnimInstance (Variables|Character|GetMesh)) "/Game/Assets/Sword_Animations/Animations/Sequence/01_Idle/AM_Idle_To_Idle_Combat_Seq.AM_Idle_To_Idle_Combat_Seq" 1.0 "MontageLength" 0.0 true)
        (bind _visible (Timeline|WeaponVisibleTimeline Play)
          (:Update
            (Rendering|Material|SetScalarParameterValue (Variables|Material|GetWeaponSkinMatDynamic) "Appearance" _visible :!class /Script/Engine.MaterialInstanceDynamic))))
      (:NewEnumerator1
        (Animation|Montage|MontagePlay (Components|SkeletalMesh|GetAnimInstance (Variables|Character|GetMesh)) "/Game/Assets/Sword_Animations/Animations/Sequence/01_Idle/AM_Idle_Combat_To_Idle_Seq.AM_Idle_Combat_To_Idle_Seq" 1.0 "MontageLength" 0.0 true)
        (Timeline|WeaponVisibleTimeline Reverse)))))

(event Input|ActionEvents|InputActionRun
  (params (Key :type Key%20Structure))
  (bind _charactermovement (Variables|Character|GetCharacterMovement))
  (:Pressed
    (Variables|Action|SetbIsRunning true)
    (Variables|/Script/Engine.CharacterMovementComponent|SetMaxWalkSpeed _charactermovement 6e+02))
  (:Released
    (Variables|Action|SetbIsRunning false)
    (Variables|/Script/Engine.CharacterMovementComponent|SetMaxWalkSpeed _charactermovement 1.8e+02)))

(event Custom|AttackTrace
  ;[0 0.4511 1] 产生伤害射线检测
  (if (Variables|Action|GetbIsAttacking)
    (CallFunction|AttackHitLogic)
    (else
      (Utilities|Time|ClearandInvalidateTimerbyHandle (Variables|Action|GetAttackTimerHandle)))))

(event Custom|AttackHitLogic
  (bind _saber (Variables|Default|GetSaber))
  ;[0.5255 1 0.291] 伤害射线产生碰撞检测逻辑
  (bind (_outhit _returnvalue) (Collision|BoxTraceByChannel (Transformation|GetSocketLocation _saber "HitStart") (Transformation|GetSocketLocation _saber "HitEnd") "5.000000,5.000000,5.000000" "0, 0, 0" "TraceTypeQuery3" false (Utilities|Array|MakeArray self) "None" true "(R=1.000000,G=0.152706,B=0.000000,A=1.000000)" "(R=0.000000,G=1.000000,B=0.000000,A=1.000000)" 2.0))
  (if _returnvalue
    (if (not (Utilities|Array|ContainsItem (Variables|Default|GetHitActors) (.HitActor (Collision|BreakHitResult _outhit))))
      (Utilities|Array|Add (Variables|Default|GetHitActors) (.HitActor (Collision|BreakHitResult _outhit)))
      (Utilities|FlowControl|Sequence
        (:then_0
          (if (Pawn|IsPlayerControlled)
            (CallFunction|PlayAttackDayton)
            (CameraShakes|StartCameraShake (Game|GetPlayerCameraManager 0) "/Game/Assets/Blueprint/Util/CameraShake/CS_AttackShake.CS_AttackShake_C" 1.0 "CameraLocal" "0, 0, 0")))
        (:then_1
          (Niagara|SpawnSystematLocation "/Game/AdvancedMagicFX12/particles/Niagara/NS_ky_hit_thunder.NS_ky_hit_thunder" (.ImpactPoint (Collision|BreakHitResult _outhit)) (Math|Conversions|RotationFromXVector (.ImpactNormal (Collision|BreakHitResult _outhit)))))
        (:then_2
          (if (Pawn|IsPlayerControlled)
            ;[0.289 1 0.1465] 击打锁定目标
            (if (Utilities|Array|ContainsItem (Variables|Default|GetLockTargetActors) (Utilities|Array|Get(acopy) (Variables|Default|GetHitActors)))
              (Variables|Default|SetLockTargetIndex (Utilities|Array|FindItem (Variables|Default|GetLockTargetActors) (Utilities|Array|Get(acopy) (Variables|Default|GetHitActors))))
              (CallFunction|PlayHitAnimation (.AsCharacter (Utilities|Casting|CastToCharacter (Utilities|Array|Get(acopy) (Variables|Default|GetLockTargetActors) (Variables|Default|GetLockTargetIndex)))) (.ImpactNormal (Collision|BreakHitResult _outhit)) :!pinned true :!label _label) ; 播放受击动画
              (UI|SwitchLockTargetUI)
              (else
                (Variables|Default|SetLockTargetIndex 0)))
            (else
              (goto _label))))))))

(event Custom|PlayAttackDayton
  ;[0.8501 1 0] 顿帧效果
  (Animation|Montage|MontageSetPlayRate (Components|SkeletalMesh|GetAnimInstance (Variables|Character|GetMesh)) (Utilities|Array|Get(acopy) (Variables|Action|GetAttackMontages) (Variables|Action|GetMontageIndex)) 0.3)
  (Utilities|FlowControl|Delay 0.1)
  (Animation|Montage|MontageSetPlayRate (Components|SkeletalMesh|GetAnimInstance (Variables|Character|GetMesh)) (Utilities|Array|Get(acopy) (Variables|Action|GetAttackMontages) (Variables|Action|GetMontageIndex)) 1.0))

(event EventSetIsAttacking
  (params (IsAttacking :type Boolean))
  (Variables|Action|SetbIsAttacking IsAttacking))

(event EventSetCanCombo
  (params (CanCombo :type Boolean))
  (Variables|Action|SetbCanCombo CanCombo))

(event EventEventAttack
  (switch Utilities|FlowControl|Switch|SwitchonE_CharacterState (Variables|Action|State|GetCurrentState)
    (:NewEnumerator1
      (if (Variables|Action|GetbCanCombo)
        (Math|Integer|IncrementInt (Variables|Action|GetMontageIndex)
          (:%20%20
            _))
        (else
          (Variables|Action|SetMontageIndex 0)))
      (Animation|Montage|MontagePlay (Components|SkeletalMesh|GetAnimInstance (Variables|Character|GetMesh)) (Utilities|Array|Get(acopy) (.ComboAnimMontages (Utilities|Struct|BreakS_ComboAnimations (Utilities|Array|Get(acopy) (Variables|Default|GetComboAnimations) (Variables|Default|GetComboIndex)))) (Variables|Action|GetMontageIndex)) 1.0 "MontageLength" 0.0 true)
      (bind _returnvalue (Utilities|Time|SetTimerbyEvent (EventDispatchers|CreateEvent :!event Custom|AttackTrace) 0.012 true 0.13))
      (Variables|Action|SetAttackTimerHandle _returnvalue))))

(event Input|ActionEvents|InputActionAttack
  (params (Key :type Key%20Structure :default "None"))
  (:Pressed
    (Variables|Action|SetbAttackKeyDown true)
    (if (Game|Player|IsInputKeyDown (.AsPlayer%20Controller (Utilities|Casting|CastToPlayerController (Pawn|GetController))) "W")
      (Variables|Default|SetComboIndex 1)
      (else
        (Variables|Default|SetComboIndex 0)))
    (if (not (Variables|Action|GetbIsAttacking))
      (CallFunction|EventAttack)))
  (:Released
    (Variables|Action|SetbAttackKeyDown false)))

(event Input|KeyboardEvents|AnyKey
  (params (Key :type Key%20Structure :default "None")))

(event Input|ActionEvents|InputActionSwitchLockTarget
  (params (Key :type Key%20Structure :default "None"))
  (:Pressed
    (if (Utilities|IsValidLockTargetArray)
      (Math|Integer|IncrementInt (Variables|Default|GetLockTargetIndex)
        (:%20%20
          (if (>= (Variables|Default|GetLockTargetIndex) (Utilities|Array|Length (Variables|Default|GetLockTargetActors)))
            (Variables|Default|SetLockTargetIndex 0))
          (UI|SwitchLockTargetUI))))))

(event Input|ActionEvents|InputActionRoll
  (params (Key :type Key%20Structure :default "None"))
  (bind _angle (CallFunction|CalculateRollDirection))
  (:Pressed
    (if (Variables|Action|GetbCanRoll)
      (Variables|Action|SetbCanRoll false)
      (if (Math|Float|InRange(Float) _angle -45.0 45.0 false false)
        (Variables|Action|State|SetRollDirection "NewEnumerator0")
        (elif (Math|Float|InRange(Float) _angle -135.0 -45.0 false)
          (Variables|Action|State|SetRollDirection "NewEnumerator2")
          (elif (Math|Float|InRange(Float) _angle 45.0 135.0 true false)
            (Variables|Action|State|SetRollDirection "NewEnumerator3")
            (else
              (Variables|Action|State|SetRollDirection "NewEnumerator1")))))
      (bind _returnvalue (Animation|Montage|MontagePlay (Components|SkeletalMesh|GetAnimInstance (Variables|Character|GetMesh)) (Utilities|Select :Index (Variables|Action|State|GetRollDirection) :NewEnumerator0 "/Game/Assets/Sword_Animations/Animations/Sequence/07_Roll/01_Roll/AM_Roll_F_0_Seq.AM_Roll_F_0_Seq" :NewEnumerator1 "/Game/Assets/Sword_Animations/Animations/Sequence/07_Roll/01_Roll/AM_Roll_B_180_Seq.AM_Roll_B_180_Seq" :NewEnumerator2 "/Game/Assets/Sword_Animations/Animations/Sequence/07_Roll/01_Roll/AM_Roll_L_90_Seq.AM_Roll_L_90_Seq" :NewEnumerator3 "/Game/Assets/Sword_Animations/Animations/Sequence/07_Roll/01_Roll/AM_Roll_R_90_Seq.AM_Roll_R_90_Seq") 1.0 "MontageLength" 0.0 true))
      (Utilities|FlowControl|Delay _returnvalue)
      (Variables|Action|SetbCanRoll true))))